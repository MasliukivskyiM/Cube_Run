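; BP_Cube is the player cube in an endless-runner style game, steered left and right while moving forward automatically.
; Tick derives score from X position, applies manual downward movement with a swept offset and adds forward input, while Canmove is true for movement.
; Hitting an "obstacle"-tagged actor stops movement and reloads the level after a delay, a path shared with RestartLvl.
; It also creates the score widget and opens the pause menu.
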(event `EnhancedInput|/Game/BluePrintsCube/Actions/IA_MoveLeft`
  (params (ActionValue :type "Float (double-precision)") (ElapsedSeconds :type "Float (double-precision)") (TriggeredSeconds :type "Float (double-precision)") (InputAction :type "InputAction Object Reference" :default "/Game/BluePrintsCube/Actions/IA_MoveLeft.IA_MoveLeft"))
  ; Move LEft
  (:`Triggered`
    (if (`self.canmove?`)
      (`self.AddMovementInput` (`KismetMathLibrary.NegateVector` (`SceneComponent.GetRightVector` (`self.Cube`))) (`self.SpeedRight`)))))

(event `EnhancedInput|/Game/BluePrintsCube/Actions/IA_MoveRight`
  (params (ActionValue :type "Float (double-precision)") (ElapsedSeconds :type "Float (double-precision)") (TriggeredSeconds :type "Float (double-precision)") (InputAction :type "InputAction Object Reference" :default "/Game/BluePrintsCube/Actions/IA_MoveRight.IA_MoveRight"))
  ; Move Right
  (:`Triggered`
    (if (`self.canmove?`)
      (`self.AddMovementInput` (`SceneComponent.GetRightVector` (`self.Cube`)) (`self.SpeedRight`)))))

(event `self.ReceiveTick`
  (params (DeltaSeconds :type "Float (single-precision)"))
  (bind _returnvalue_x (`KismetMathLibrary.BreakVector` (`SceneComponent.K2_GetComponentLocation` (`self.Cube`))))
  ; Display numbers of score
  (set `self.Score` (`KismetMathLibrary.FTrunc` (/ _returnvalue_x 100.0)))
  (if (`self.canmove?`)
    (`self.K2_AddActorWorldOffset` (* (`KismetMathLibrary.NegateVector` (`SceneComponent.GetUpVector` (`self.Cube`))) (* (`self.FallSpeed`) (`GameplayStatics.GetWorldDeltaSeconds`))) true)
    (`|ExecutionSequence`
      (:`then_0`
        ; move Forward
        (if (`self.canmove?`)
          (`self.AddMovementInput` (`SceneComponent.GetForwardVector` (`self.Cube`)) (`self.SpeedForward`)))))))

(event `self.Cube.OnComponentHit`
  (params (HitComponent :type "PrimitiveComponent Object Reference") (OtherActor :type "Actor Object Reference") (OtherComp :type "PrimitiveComponent Object Reference") (NormalImpulse :type "Vector Structure") (Hit :type "HitResult Structure (by ref)"))
  (if (`self.ActorHasTag` OtherActor "obstacle")
    (set `self.canmove?` false)
    (`KismetSystemLibrary.Delay` (`self.RestartDelay`) :!label _label)
    ; Restart lvl if cube hit obstacle
    (bind _returnvalue (`GameplayStatics.GetCurrentLevelName` true))
    (`GameplayStatics.OpenLevel` (`KismetStringLibrary.Conv_StringToName` _returnvalue))))

(event `RestartLvl`
  (goto _label))

(event `self.ReceiveBeginPlay`
  (bind _returnvalue (`GameplayStatics.GetPlayerController` 0))
  ; Dont display mouse coursor in game
  (`WidgetBlueprintLibrary.SetInputMode_GameOnly` _returnvalue)
  (set `PlayerController.bShowMouseCursor` false _returnvalue)
  ; Display score
  (bind _returnvalue_2 (`|CreateWidget` "/Game/BluePrintsCube/WB_Score.WB_Score_C"))
  (`UserWidget.AddToViewport` _returnvalue_2 0))

(event `EnhancedInput|/Game/BluePrintsCube/Actions/IA_Pause`
  (params (ActionValue :type Boolean) (ElapsedSeconds :type "Float (double-precision)") (TriggeredSeconds :type "Float (double-precision)") (InputAction :type "InputAction Object Reference" :default "/Game/BluePrintsCube/Actions/IA_Pause.IA_Pause"))
  (bind _returnvalue (`GameplayStatics.GetPlayerController` 0))
  (:`Started`
    (bind _returnvalue_2 (`|CreateWidget` "/Game/BluePrintsCube/WB_PauseMenu.WB_PauseMenu_C"))
    (`UserWidget.AddToViewport` _returnvalue_2 0)
    (set `PlayerController.bShowMouseCursor` true _returnvalue)
    (`WidgetBlueprintLibrary.SetInputMode_UIOnlyEx` _returnvalue null)
    (`GameplayStatics.SetGamePaused` true)))

(fn `UserConstructionScript`)